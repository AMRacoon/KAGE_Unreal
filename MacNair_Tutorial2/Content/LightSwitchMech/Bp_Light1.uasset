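; Bp_Light1 is a light Blueprint whose RectLight follows the on/off state of a linked light switch.
; On BeginPlay and in SwitchLight, it casts SwitchActor to Bp_LightSwitch and sets the RectLight's visibility from IsOn.
; SwitchLight has no caller within this Blueprint.
; A separate TurnOff zeroes the light's intensity, while TurnOn is empty, with its intensity call left disconnected.
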(event `self.ReceiveBeginPlay`
  (bind _asbp_light_switch (cast `/Game/LightSwitchMech/Bp_LightSwitch` (`self.SwitchActor`)))
  (`SceneComponent.SetVisibility` (`self.RectLight`) (`/Game/LightSwitchMech/Bp_LightSwitch.IsOn` _asbp_light_switch) false))

(fn `SwitchLight`
  (bind _asbp_light_switch (cast `/Game/LightSwitchMech/Bp_LightSwitch` (`self.SwitchActor`)))
  (`SceneComponent.SetVisibility` (`self.RectLight`) (`/Game/LightSwitchMech/Bp_LightSwitch.IsOn` _asbp_light_switch) false))

(fn `TurnOff`
  (`LightComponent.SetIntensity` (`self.RectLight`) 0.0))

(fn `TurnOn`)

(fn `UserConstructionScript`)